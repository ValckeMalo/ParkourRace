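; Game mode for a parkour race that tracks the current checkpoint, respawns the player character and handles level completion.
; Respawn spawns a new character at the saved checkpoint, falling back to a PlayerStart, with a possess step for player controller 0.
; Winning plays the HUD's match-over animation, whose finish event loads Level 2 after the first level or the menu otherwise.
; Pause toggling is forwarded to the race HUD cached at BeginPlay.
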(event Custom|Anim%20Fnish
  (if (== (Variables|Default|GetLevelIndex) 0)
    (Game|OpenLevel(byObjectReference) "/Game/Levels/L_Level2.L_Level2")
    (else
      (Game|OpenLevel(byObjectReference) "/Game/Levels/L_Menu.L_Menu"))))

(event EventBeginPlay
  (bind _ashud_parkour_race (Utilities|Casting|CastToHUD_ParkourRace (HUD|GetHUD (Game|GetPlayerController 0))))
  (Variables|Default|SetHUD%20Parkour%20Race _ashud_parkour_race))

(event EventWin
  (params (level :type Integer))
  (bind _hud_parkour_race (Variables|Default|GetHUD%20Parkour%20Race))
  (bind _hud (Variables|/Game/Blueprints/Core/HUD_ParkourRace.HUD_ParkourRace_C|GetHUD _hud_parkour_race))
  (bind _matchoveranim (Variables|/Game/Blueprints/UI/W_HUDWidget.W_HUDWidget_C|GetMatchOverAnim _hud))
  (Variables|Default|SetLevelIndex level)
  (Default|PlayAnim _hud _matchoveranim 1.0)
  (Class|UserWidget|BindtoAnimationEvent _hud _matchoveranim (delegate Custom|Anim%20Fnish) "Finished" "None"))

(event EventUpdateCheckpoint
  (params (New%20Checkpoint :type BP%20Checkpoint%20Object%20Reference))
  (Variables|Default|SetCurrentCheckpoint New%20Checkpoint))

(fn ConstructionScript)

(fn RespawnChara
  (Utilities|IsValid (Variables|Default|GetCurrentCheckpoint)
    (:Is%20Valid
      (bind _returnvalue (Game|SpawnActorfromClass "/Game/Blueprints/Core/P_MainChara.P_MainChara_C" (Transformation|GetActorTransform (Variables|Default|GetCurrentCheckpoint)) "Undefined" "MultiplyWithRoot" 0 0)))
    (:Is%20Not%20Valid
      (bind _returnvalue_2 (Actor|GetActorOfClass "/Script/Engine.PlayerStart"))
      (Utilities|IsValid _returnvalue_2
        (:Is%20Valid
          (Game|SpawnActorfromClass "/Game/Blueprints/Core/P_MainChara.P_MainChara_C" (Transformation|GetActorTransform _returnvalue_2) "Undefined" "MultiplyWithRoot" 0 0)))))
  (Pawn|Possess (Game|GetPlayerController 0) _returnvalue))

(fn TogglePause
  (Default|TogglePauseMenu (Variables|Default|GetHUD%20Parkour%20Race)))