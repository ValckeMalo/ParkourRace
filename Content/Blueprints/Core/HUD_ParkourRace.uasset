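; HUD Blueprint for the parkour race mode that shows the race HUD and handles the pause menu.
; On BeginPlay it creates a W_HUDWidget, adds it to the viewport and plays its GoAnim.
; TogglePauseMenu flips the paused state, switches the widget switcher between its two pages, shows or hides the mouse cursor and pauses or resumes the game.
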(event EventBeginPlay
  (bind _returnvalue (UserInterface|CreateWidget "/Game/Blueprints/UI/W_HUDWidget.W_HUDWidget_C"))
  (bind _output_get (Variables|Default|SetHUD _returnvalue))
  (UserInterface|Viewport|AddtoViewport _output_get 0)
  (Default|PlayAnim (Variables|Default|GetHUD) (Variables|/Game/Blueprints/UI/W_HUDWidget.W_HUDWidget_C|GetGoAnim (Variables|Default|GetHUD)) 1.0))

(fn ConstructionScript)

(fn TogglePauseMenu
  (bind _hud (Variables|Default|GetHUD))
  (bind _widgetswitcher (Variables|/Game/Blueprints/UI/W_HUDWidget.W_HUDWidget_C|GetWidgetSwitcher _hud))
  (bind _output_get (Variables|Default|SetGame%20Paused (not (Variables|Default|GetGame%20Paused))))
  (if _output_get
    (Variables|/Script/UMG.WidgetSwitcher|SetActiveWidgetIndex _widgetswitcher 1)
    (else
      (Variables|/Script/UMG.WidgetSwitcher|SetActiveWidgetIndex _widgetswitcher 0)))
  (Variables|/Script/Engine.PlayerController|SetbShowMouseCursor (Game|GetPlayerController 0) (Variables|Default|GetGame%20Paused))
  (Game|SetGamePaused (Variables|Default|GetGame%20Paused)))