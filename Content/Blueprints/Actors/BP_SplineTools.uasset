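; BP_SplineTools is an actor that procedurally builds a fence along its spline from the Construction Script.
; BuildFence loops over every spline point, adding a static mesh at the point's local transform, without spline scale.
; It also adds a spline mesh from each point to the next index, using local locations and tangents to follow the curve.
; The last point also gets a segment, targeting an index past the end.
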(fn ConstructionScript
  (CallFunction|BuildFence))

(fn BuildFence
  (for _index (range 0 (- (Spline|GetNumberOfSplinePoints (Variables|Default|GetSpline)) 1))
    (AddComponent|AddStaticMeshComponent false (Spline|GetTransformatSplinePoint (Variables|Default|GetSpline) _index "Local" false))
    (bind _returnvalue (AddComponent|AddSplineMeshComponent false))
    (SplineMesh|SetStartandEnd _returnvalue (.Location (Spline|GetLocationandTangentatSplinePoint (Variables|Default|GetSpline) _index "Local")) (.Tangent (Spline|GetLocationandTangentatSplinePoint (Variables|Default|GetSpline) _index "Local")) (.Location (Spline|GetLocationandTangentatSplinePoint (Variables|Default|GetSpline) (+ _index 1) "Local")) (.Tangent (Spline|GetLocationandTangentatSplinePoint (Variables|Default|GetSpline) (+ _index 1) "Local")) true :!class /Script/Engine.SplineMeshComponent)))