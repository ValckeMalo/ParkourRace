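; BP_Checkpoint is a checkpoint actor that reports to the game mode when something overlaps its Box trigger.
; The overlap event calls UpdateCheckpointMessage on the game mode, passing itself, with no filtering of the overlapping actor.
; The construction script builds a dynamic instance of MI_CheckPoint for the Plane, driving its Color and SpeedX parameters from the actor's Color and Scalar variables.
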(event OnComponentBeginOverlap(Box)
  (params (OverlappedComponent :type Primitive%20Component%20Object%20Reference) (OtherActor :type Actor%20Object%20Reference) (OtherComp :type Primitive%20Component%20Object%20Reference) (OtherBodyIndex :type Integer) (bFromSweep :type Boolean) (SweepResult :type Hit%20Result%20Structure%20%28by%20ref%29))
  (Class|BPIPlayer|UpdateCheckpoint(Message) (Game|GetGameMode) self))

(fn ConstructionScript
  (bind _returnvalue (Rendering|Material|CreateDynamicMaterialInstance "/Game/Materials/MI_CheckPoint.MI_CheckPoint" "None" "None" :!class /Script/Engine.KismetMaterialLibrary))
  (Rendering|Material|SetVectorParameterValue _returnvalue "Color" (Variables|Default|GetColor) :!class /Script/Engine.MaterialInstanceDynamic)
  (Rendering|Material|SetScalarParameterValue _returnvalue "SpeedX" (Variables|Default|GetScalar) :!class /Script/Engine.MaterialInstanceDynamic)
  (Rendering|Material|SetMaterial (Variables|Default|GetPlane) 0 _returnvalue))